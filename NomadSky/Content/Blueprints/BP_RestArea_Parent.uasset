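; Parent rest area actor where the player sleeps to regain energy, with diminishing returns on repeat visits.
; The Sphere overlap blends the view to the bed camera and shows a prompt, while the Box overlap gates the Interact input.
; Interact runs a one-shot sleep cycle: timeline camera fade to black and back, toggled player sleep flags, then a delayed reset.
; A visit counter sets the energy gain and triggers the player's win-state UI.
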(event `self.Sphere.OnComponentBeginOverlap`
  (params (OverlappedComponent :type "PrimitiveComponent Object Reference") (OtherActor :type "Actor Object Reference") (OtherComp :type "PrimitiveComponent Object Reference") (OtherBodyIndex :type Integer) (bFromSweep :type Boolean) (SweepResult :type "HitResult Structure (by ref)"))
  ;[1 1 1] Swap between player cam and bed cam on overlaps, reset interaction for sleep cycles.
  (bind _asthird_person_character (cast `/Game/ThirdPersonCPP/Blueprints/ThirdPersonCharacter` OtherActor))
  (set `self.Player` _asthird_person_character)
  (`self.SwitchToBedCam`)
  (`/Game/ThirdPersonCPP/Blueprints/ThirdPersonCharacter.UMGBedControlPrompt` (`self.Player`)))

(event `self.Sphere.OnComponentEndOverlap`
  (params (OverlappedComponent :type "PrimitiveComponent Object Reference") (OtherActor :type "Actor Object Reference") (OtherComp :type "PrimitiveComponent Object Reference") (OtherBodyIndex :type Integer))
  ;[1 1 1] Swap between player cam and bed cam on overlaps, reset interaction for sleep cycles.
  (cast `/Game/ThirdPersonCPP/Blueprints/ThirdPersonCharacter` OtherActor)
  (`self.SwitchToPlayerCam`)
  (`/Game/ThirdPersonCPP/Blueprints/ThirdPersonCharacter.UMGRemove` (`self.Player`)))

(event `InputAction|Interact`
  (params (Key :type "Key Structure"))
  (bind _player (`self.Player`))
  (bind _player_2 (`self.Player`))
  ;[1 1 1] On overlapping box allow interact, fade screen to black and engage sleep cycle, wake after cycle ends.
  (:`Pressed`
    (`/Engine/EditorBlueprintResources/StandardMacros.Gate` true :!label _label
      (:`Exit`
        (`/Engine/EditorBlueprintResources/StandardMacros.DoOnce` false :!label _label_2
          (:`Completed`
            (`/Game/ThirdPersonCPP/Blueprints/ThirdPersonCharacter.UMGRemove` (`self.Player`))
            (`self.TrackTimesVisited`)
            (`KismetSystemLibrary.PrintString` "Hello")
            (`self.DisableInput` (`self.Player`) (`GameplayStatics.GetPlayerController` 0))
            (`KismetSystemLibrary.PrintString` "Player Chose to Sleep")
            (`self.AddRelativeEnergy`)
            (set `/Game/ThirdPersonCPP/Blueprints/ThirdPersonCharacter.wakeUp` false _player)
            (set `/Game/ThirdPersonCPP/Blueprints/ThirdPersonCharacter.bedtime` true _player)
            (bind (_direction _fadevalue) (`Timeline|FadeToBlack` :!via `PlayFromStart` :!label _label_3)
              (:`Update`
                (`PlayerCameraManager.SetManualCameraFade` :`self` (`GameplayStatics.GetPlayerCameraManager` 0) :`InFadeAmount` _fadevalue))
              (:`Finished`
                (`KismetSystemLibrary.PrintString` "Wake")
                (`KismetSystemLibrary.Delay` 1.0)
                (`self.Reverse`)
                (`self.EnableInput` (`self.Player`) (`GameplayStatics.GetPlayerController` 0))
                (set `/Game/ThirdPersonCPP/Blueprints/ThirdPersonCharacter.wakeUp` true _player_2)
                (set `/Game/ThirdPersonCPP/Blueprints/ThirdPersonCharacter.bedtime` false _player_2)
                (`KismetSystemLibrary.Delay` 0.1)
                (set `/Game/ThirdPersonCPP/Blueprints/ThirdPersonCharacter.wakeUp` false _player_2)
                (`KismetSystemLibrary.Delay` 3.0)
                (`self.Reset`)))))))))

(event `self.Box.OnComponentBeginOverlap`
  (params (OverlappedComponent :type "PrimitiveComponent Object Reference") (OtherActor :type "Actor Object Reference") (OtherComp :type "PrimitiveComponent Object Reference") (OtherBodyIndex :type Integer) (bFromSweep :type Boolean) (SweepResult :type "HitResult Structure (by ref)"))
  ;[1 1 1] On overlapping box allow interact, fade screen to black and engage sleep cycle, wake after cycle ends.
  (cast `/Game/ThirdPersonCPP/Blueprints/ThirdPersonCharacter` OtherActor)
  (goto _label :!via `Open`))

(event `Reset`
  ;[1 1 1] On overlapping box allow interact, fade screen to black and engage sleep cycle, wake after cycle ends.
  (`|ExecutionSequence`
    (:`then_0`
      (goto _label_2 :!via `Reset`))
    (:`then_1`
      (goto _label_4 :!via `Reset`))))

(event `Reverse`
  ;[1 1 1] On overlapping box allow interact, fade screen to black and engage sleep cycle, wake after cycle ends.
  (`/Engine/EditorBlueprintResources/StandardMacros.DoOnce` false :!label _label_4
    (:`Completed`
      (goto _label_3 :!via `ReverseFromEnd`))))

(event `self.Box.OnComponentEndOverlap`
  (params (OverlappedComponent :type "PrimitiveComponent Object Reference") (OtherActor :type "Actor Object Reference") (OtherComp :type "PrimitiveComponent Object Reference") (OtherBodyIndex :type Integer))
  ;[1 1 1] On overlapping box allow interact, fade screen to black and engage sleep cycle, wake after cycle ends.
  (cast `/Game/ThirdPersonCPP/Blueprints/ThirdPersonCharacter` OtherActor)
  (goto _label :!via `Close`))

(fn `AddRelativeEnergy`
  (bind _player (`self.Player`))
  (bind _energyadded (`self.EnergyAdded`))
  (bind _returnvalue (+ (`/Game/ThirdPersonCPP/Blueprints/ThirdPersonCharacter.Energy` _player) _energyadded))
  (bind _output_get (set `self.TimesVisitedCount` (+ (`self.TimesVisitedCount`) 1)))
  (switch `int` _output_get
    (:`1`
      (set `self.EnergyAdded` 80.0))
    (:`2`
      (set `self.EnergyAdded` 50.0))
    (:`3`
      (set `self.EnergyAdded` 20.0))
    (:`4`
      (set `self.EnergyAdded` 5.0)))
  (set `/Game/ThirdPersonCPP/Blueprints/ThirdPersonCharacter.Energy` _returnvalue _player)
  (`KismetSystemLibrary.PrintString` (`KismetStringLibrary.Concat_StrStr` "Added Energy: " (`KismetStringLibrary.Conv_DoubleToString` _energyadded)) true true (struct :`R` 0.209461 :`G` 1.0 :`B` 0.005113 :`A` 1.0))
  (if (> _returnvalue 100.0)
    (set `/Game/ThirdPersonCPP/Blueprints/ThirdPersonCharacter.Energy` 100.0 _player)))

(fn `SwitchToBedCam`
  (bind _returnvalue (`GameplayStatics.GetPlayerController` 0))
  (`PlayerController.SetViewTargetWithBlend` _returnvalue self 1.0 "VTBlend_Linear" 0.0 true)
  (`self.EnableInput` _returnvalue))

(fn `SwitchToPlayerCam`
  (bind _returnvalue (`GameplayStatics.GetPlayerController` 0))
  (`PlayerController.SetViewTargetWithBlend` _returnvalue (`self.Player`) 1.0 "VTBlend_Linear" 0.0 true)
  (`self.DisableInput` _returnvalue))

(fn `TrackTimesVisited`
  (if (== (`self.TimesVisitedCount`) 5)
    (`/Game/ThirdPersonCPP/Blueprints/ThirdPersonCharacter.UMGWinState` (`self.Player`) "")))

(fn `UserConstructionScript`)