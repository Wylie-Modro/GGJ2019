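; Parent Blueprint for a point of interest that lets the player view it through an orbiting camera.
; Overlapping InterestArea enables input and shows a prompt; a looping timeline spins the SpringArm.
; Interact flip-flops a blended view target between POI and player, toggling player input, with DoOnce and delays guarding transitions.
; CheckIfVisited passes the name to the player's win-state UI if visited.
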(event `self.InterestArea.OnComponentBeginOverlap`
  (params (OverlappedComponent :type "PrimitiveComponent Object Reference") (OtherActor :type "Actor Object Reference") (OtherComp :type "PrimitiveComponent Object Reference") (OtherBodyIndex :type Integer) (bFromSweep :type Boolean) (SweepResult :type "HitResult Structure (by ref)"))
  ;[1 1 1] Enable/Disable input interaction on this blueprint
  (bind _asthird_person_character (cast `/Game/ThirdPersonCPP/Blueprints/ThirdPersonCharacter` OtherActor))
  (bind _output_get (set `self.Player` _asthird_person_character))
  (`self.EnableInput` (`GameplayStatics.GetPlayerController` 0))
  (`/Game/ThirdPersonCPP/Blueprints/ThirdPersonCharacter.UMGPOIControlPrompt` _output_get))

(event `self.InterestArea.OnComponentEndOverlap`
  (params (OverlappedComponent :type "PrimitiveComponent Object Reference") (OtherActor :type "Actor Object Reference") (OtherComp :type "PrimitiveComponent Object Reference") (OtherBodyIndex :type Integer))
  ;[1 1 1] Enable/Disable input interaction on this blueprint
  (cast `/Game/ThirdPersonCPP/Blueprints/ThirdPersonCharacter` OtherActor)
  (`self.DisableInput` (`GameplayStatics.GetPlayerController` 0))
  (`/Game/ThirdPersonCPP/Blueprints/ThirdPersonCharacter.UMGRemove` (stale `self.InterestArea.OnComponentBeginOverlap` _output_get)))

(event `self.ReceiveBeginPlay`
  ;[1 1 1] On beginplay start RotationAnimation of camera around the parent(Mesh), replay to loop when finished
  (bind (_direction _rotationrate) (`Timeline|RotationAnim` :!via `PlayFromStart` :!label _label)
    (:`Update`
      (`SceneComponent.K2_SetRelativeRotation` (`self.SpringArm`) (`KismetMathLibrary.MakeRotator` 0.0 0.0 _rotationrate) false false))
    (:`Finished`
      (`self.Replay`))))

(event `Replay`
  ;[1 1 1] On beginplay start RotationAnimation of camera around the parent(Mesh), replay to loop when finished
  (goto _label :!via `PlayFromStart`))

(event `InputAction|Interact`
  (params (Key :type "Key Structure"))
  (bind _returnvalue (`GameplayStatics.GetPlayerController` 0))
  (bind _returnvalue_2 (`GameplayStatics.GetPlayerController` 0))
  (bind _player (`self.Player`))
  (bind _player_2 (`self.Player`))
  ;[1 1 1] On Interact flip flop between switching player controller camera to interest cam and back to player cam.
  (:`Pressed`
    (`/Engine/EditorBlueprintResources/StandardMacros.DoOnce` false :!label _label_2
      (:`Completed`
        (`/Game/ThirdPersonCPP/Blueprints/ThirdPersonCharacter.UMGRemove` _player_2)
        (`/Engine/EditorBlueprintResources/StandardMacros.FlipFlop`
          (:`A`
            (set `/Game/ThirdPersonCPP/Blueprints/ThirdPersonCharacter.AtPOI?` true _player_2)
            (`PlayerController.SetViewTargetWithBlend` _returnvalue self 2.0 "VTBlend_Cubic" 0.0 false)
            (`self.DisableInput` _player _returnvalue_2)
            (`KismetSystemLibrary.Delay` 2.0))
          (:`B`
            (set `/Game/ThirdPersonCPP/Blueprints/ThirdPersonCharacter.AtPOI?` false _player_2)
            (`PlayerController.SetViewTargetWithBlend` _returnvalue (`self.Player`) 2.0 "VTBlend_Cubic" 0.0 false)
            (`self.EnableInput` _player _returnvalue_2)
            (`KismetSystemLibrary.Delay` 2.0)))
        (`self.Reset`)))))

(event `Reset`
  ;[1 1 1] On Interact flip flop between switching player controller camera to interest cam and back to player cam.
  (goto _label_2 :!via `Reset`))

(fn `CheckIfVisited`
  ;[1 1 1] Draw Symbol with CheckMark.
  (if (`self.bWasVisited?`)
    (`/Game/ThirdPersonCPP/Blueprints/ThirdPersonCharacter.UMGWinState` (`self.Player`) (`self.Name`))))

(fn `UserConstructionScript`)