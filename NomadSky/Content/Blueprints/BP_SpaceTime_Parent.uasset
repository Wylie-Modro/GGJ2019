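; Parent actor for a biome zone that tracks how long the player spends inside it and identifies the player's home biome on death.
; Sphere overlap with a ThirdPersonCharacter opens and closes a Gate, letting a one-second Delay on Tick accumulate and print TimeSpent.
; When PlayerDied fires, HomeBiome prints this biome's name only if its time exceeds both referenced sibling biomes.
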(event `self.ReceiveBeginPlay`
  (bind _outactors (`GameplayStatics.GetAllActorsOfClass` "/Game/ThirdPersonCPP/Blueprints/ThirdPersonCharacter.ThirdPersonCharacter_C"))
  (for _array_element _outactors
    (bind _output_get (set `self.Player` _array_element))
    (add `/Game/ThirdPersonCPP/Blueprints/ThirdPersonCharacter.PlayerDied` _output_get (delegate `CheckTimeSpent`))))

(event `CheckTimeSpent`
  (`self.HomeBiome`))

(event `self.ReceiveTick`
  (params (DeltaSeconds :type "Float (single-precision)"))
  (`KismetSystemLibrary.Delay` 1.0)
  (`/Engine/EditorBlueprintResources/StandardMacros.Gate` true :!label _label
    (:`Exit`
      (bind _output_get (set `self.TimeSpent` (+ (`self.TimeSpent`) 1.0)))
      (`KismetSystemLibrary.PrintString` (`KismetStringLibrary.Concat_StrStr` (`KismetTextLibrary.Conv_TextToString` (`self.BiomeName`)) " :" (`KismetStringLibrary.Conv_DoubleToString` _output_get))))))

(event `OpenGate`
  (goto _label :!via `Open`))

(event `CloseGate`
  (goto _label :!via `Close`))

(event `self.Sphere.OnComponentBeginOverlap`
  (params (OverlappedComponent :type "PrimitiveComponent Object Reference") (OtherActor :type "Actor Object Reference") (OtherComp :type "PrimitiveComponent Object Reference") (OtherBodyIndex :type Integer) (bFromSweep :type Boolean) (SweepResult :type "HitResult Structure (by ref)"))
  (cast `/Game/ThirdPersonCPP/Blueprints/ThirdPersonCharacter` OtherActor)
  (`self.OpenGate`))

(event `self.Sphere.OnComponentEndOverlap`
  (params (OverlappedComponent :type "PrimitiveComponent Object Reference") (OtherActor :type "Actor Object Reference") (OtherComp :type "PrimitiveComponent Object Reference") (OtherBodyIndex :type Integer))
  (cast `/Game/ThirdPersonCPP/Blueprints/ThirdPersonCharacter` OtherActor)
  (`self.CloseGate`))

(fn `HomeBiome`
  (`/Engine/EditorBlueprintResources/StandardMacros.CompareFloat` (`self.TimeSpent`) (`/Game/Blueprints/BP_SpaceTime_Parent.TimeSpent` (`self.OtherBiome1`))
    (:`>`
      (`/Engine/EditorBlueprintResources/StandardMacros.CompareFloat` (`self.TimeSpent`) (`/Game/Blueprints/BP_SpaceTime_Parent.TimeSpent` (`self.OtherBiome2`))
        (:`>`
          (`KismetSystemLibrary.PrintText` (`self.BiomeName`)))))))

(fn `UserConstructionScript`)